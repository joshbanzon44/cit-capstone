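; BP_MenuWizard is the wizard character shown in the main menu, previewing the colors chosen in the menu.
; One tick after BeginPlay it puts a dynamic instance of MI_Wizard on its skeletal mesh.
; It then binds to the MenuController widget's hair, inner clothes and outer clothes color events, each of which writes the matching vector parameter on that material.
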(event Custom|OnHairColorUpdate
  (params (Color :type Linear%20Color%20Structure))
  (Rendering|Material|SetVectorParameterValue (Variables|Default|GetDynMat) "Hair" Color :!class /Script/Engine.MaterialInstanceDynamic))

(event Custom|OnInnerClothesColorUpdate
  (params (Color :type Linear%20Color%20Structure))
  (Rendering|Material|SetVectorParameterValue (Variables|Default|GetDynMat) "InnerCloth" Color :!class /Script/Engine.MaterialInstanceDynamic))

(event Custom|OnOuterClothesColorUpdate
  (params (Color :type Linear%20Color%20Structure))
  (Rendering|Material|SetVectorParameterValue (Variables|Default|GetDynMat) "OuterClothes" Color :!class /Script/Engine.MaterialInstanceDynamic))

(event EventBeginPlay
  (Utilities|FlowControl|DelayUntilNextTick)
  (bind _returnvalue (Rendering|Material|CreateDynamicMaterialInstance "/Game/Materials/Wizard/MI_Wizard.MI_Wizard" "None" "None" :!class /Script/Engine.KismetMaterialLibrary))
  (bind _output_get (Variables|Default|SetDynMat _returnvalue))
  (Rendering|Material|SetMaterial (Variables|Default|GetSkeletalMeshComponent0) 0 _output_get)
  (bind _asmenu_controller (Utilities|Casting|CastToMenuController (Game|GetPlayerController 0)))
  (EventDispatchers|BindEventtoUpdateHairColor (Variables|/Game/MainMenu/MenuController.MenuController_C|GetMenuWidget _asmenu_controller) (delegate Custom|OnHairColorUpdate))
  (EventDispatchers|BindEventtoUpdateInnerClothesColor (Variables|/Game/MainMenu/MenuController.MenuController_C|GetMenuWidget _asmenu_controller) (delegate Custom|OnInnerClothesColorUpdate))
  (EventDispatchers|BindEventtoUpdateOuterClothesColor (Variables|/Game/MainMenu/MenuController.MenuController_C|GetMenuWidget _asmenu_controller) (delegate Custom|OnOuterClothesColorUpdate)))

(event Collision|EventActorBeginOverlap
  (params (OtherActor :type Actor%20Object%20Reference)))

(event EventTick
  (params (DeltaSeconds :type Float%20%28single-precision%29)))

(fn ConstructionScript)