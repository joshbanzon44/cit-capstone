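; BP_ChestMonster is an enemy Blueprint that drives its behavior toward the player through a steering behavior list, extending its parent's logic.
; On BeginPlay it clears the list and calls AddSteering, which adds one player-targeted behavior after a given delay.
; Attack runs the parent attack, then clears steering and restores it after a short pause.
; A second steering entry is left unconnected and never runs.
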(event Custom|AddSteering
  (params (Delay :type Float%20%28double-precision%29))
  (Utilities|FlowControl|Delay Delay)
  (Utilities|Array|Add (Variables|Default|GetSteeringBehaviors) (Utilities|Struct|MakeSteeringBehaviorStruct "NewEnumerator2" 0.2 (Variables|Default|GetPlayer) 1e+03 5e+02 2e+01 0.0)))

(event EventBeginPlay
  (|CallParentFunction)
  (Utilities|Array|Clear (Variables|Default|GetSteeringBehaviors))
  (CallFunction|AddSteering 0.0))

(event EventTick
  (params (DeltaSeconds :type Float%20%28single-precision%29))
  (|CallParentFunction DeltaSeconds))

(fn ConstructionScript
  (|CallParentFunction))

(fn Attack
  (|CallParentFunction)
  (Utilities|Array|Clear (Variables|Default|GetSteeringBehaviors))
  (CallFunction|AddSteering 1.5))