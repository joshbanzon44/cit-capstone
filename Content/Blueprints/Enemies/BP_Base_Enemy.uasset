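; Base enemy Blueprint that levels itself up to PlayerLevel on spawn, attacks when the player is within range and plays periodic audio.
; An AC_StatSystem component holds its stats, takes damage and feeds a health bar turned toward the player each tick.
; Attacks set DoAttack, with a randomized cooldown timer on an empty function.
; At zero health it adds stat rewards to the player, calls Defeated and destroys itself.
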(event OnZeroHealth(AC_StatSystem)
  (bind _ac_statsystem (Variables|Default|GetAC_StatSystem))
  (bind _player (Variables|Default|GetPlayer))
  (bind _ac_statsystem_2 (Variables|/Game/Blueprints/BP_Player.BP_Player_C|GetAC_StatSystem _player))
  (Default|AddStatValue _ac_statsystem_2 "NewEnumerator1" (.Value (Default|GetStat _ac_statsystem "NewEnumerator11")))
  (Default|AddStatValue _ac_statsystem_2 "NewEnumerator13" (.Value (Default|GetStat _ac_statsystem "NewEnumerator13")))
  (Default|CallDefeated)
  (Actor|DestroyActor))

(event Custom|OnAttack
  (bind _attackdelay (Variables|Default|GetAttackDelay))
  (if (not (Utilities|Time|IsTimerActivebyHandle (Variables|Default|GetTimer)))
    (Variables|Default|SetDoAttack true)
    (Utilities|FlowControl|Delay (Variables|Default|GetAttackAnimationDelay))
    (CallFunction|Attack)
    (bind _returnvalue (Utilities|Time|SetTimerbyFunctionName 0 "NULL" (Math|Random|RandomFloatinRange _attackdelay (+ _attackdelay 2.0))))
    (Variables|Default|SetTimer _returnvalue)
    (Utilities|FlowControl|DelayUntilNextTick)
    (Variables|Default|SetDoAttack false)))

(event Custom|PlaySound
  (bind _audiocomponent (Variables|Default|GetAudioComponent))
  (if (not (Variables|Default|GetDoAttack))
    (Utilities|IsValid (Variables|/Script/Engine.AudioComponent|GetSound _audiocomponent)
      (:Is%20Valid
        (Audio|Components|Audio|Play _audiocomponent 0.0)))))

(event EventBeginPlay
  (bind _ac_statsystem (Variables|Default|GetAC_StatSystem))
  (bind _asbp_player (Utilities|Casting|CastToBP_Player (Game|Player|GetPlayerPawn 0)))
  (Variables|Default|SetPlayer _asbp_player)
  (bind _asw_health_bar (Utilities|Casting|CastToW_HealthBar (UserInterface|GetWidget (Variables|Default|GetHealthBar))))
  (Variables|Default|SetW_HealthBar _asw_health_bar)
  (CallFunction|SetStats)
  (Default|SetStatValue _ac_statsystem "NewEnumerator2" (.Value (Default|GetStat _ac_statsystem "NewEnumerator3")))
  (Utilities|Time|SetTimerbyEvent (delegate Custom|PlaySound) (Math|Random|RandomFloatinRange 5.0 1e+01) true))

(event EventTakeDamage
  (params (Amount :type Float%20%28double-precision%29))
  (bind _value (Default|SubtractStatValue (Variables|Default|GetAC_StatSystem) "NewEnumerator2" Amount))
  (Development|PrintString (Utilities|String|ToString(Float) _value)))

(event EventTick
  (params (DeltaSeconds :type Float%20%28single-precision%29))
  (bind _ac_statsystem (Variables|Default|GetAC_StatSystem))
  (|CallParentFunction 0.0)
  (Utilities|FlowControl|Sequence
    (:then_0
      (if (Variables|Default|GetRotateToFacePlayer)
        (Transformation|SetActorRotation (Math|Rotator|Lerp(Rotator) (Transformation|GetActorRotation) (Math|Rotator|FindLookatRotation (Transformation|GetWorldLocation (Variables|Default|GetEyeLocation)) (Transformation|GetActorLocation (Variables|Default|GetPlayer))) (* DeltaSeconds 5.0) true))))
    (:then_1
      (if (<= (Math|Vector|Distance(Vector) (Transformation|GetActorLocation) (Transformation|GetActorLocation (Game|Player|GetPlayerPawn 0))) (Variables|Default|GetAttackDistance))
        (CallFunction|OnAttack)))
    (:then_2
      (Transformation|SetWorldRotation (Variables|Default|GetHealthBar) (Math|Rotator|FindLookatRotation (Transformation|GetActorLocation) (Transformation|GetActorLocation (Variables|Default|GetPlayer))) false false)
      (Default|Update (Variables|Default|GetW_HealthBar) (/ (.Value (Default|GetStat _ac_statsystem "NewEnumerator2")) (.Value (Default|GetStat _ac_statsystem "NewEnumerator3")))))))

(fn ConstructionScript)

(fn DestroyOwnedComponent
  (params (Comp%20to%20Destroy :type Actor%20Component%20Object%20Reference))
  (Components|DestroyComponent Comp%20to%20Destroy))

(fn Attack
  (Variables|Default|SetDoAttack true))

(fn NULL)

(fn SetStats
  (bind _ac_statsystem (Variables|Default|GetAC_StatSystem))
  (bind _ac_statsystem_2 (Variables|Default|GetAC_StatSystem))
  (bind _value (Default|GetStat _ac_statsystem_2 "NewEnumerator0"))
  (while (> (Variables|Default|GetPlayerLevel) (Math|Float|Truncate _value))
    (Default|AddStatValue _ac_statsystem "NewEnumerator1" (.Value (Default|GetStat _ac_statsystem "NewEnumerator7"))))
  (Development|PrintString (Utilities|String|Append "level: " (Utilities|String|ToString(Float) _value))))