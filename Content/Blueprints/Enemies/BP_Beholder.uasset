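; Beholder enemy that steers relative to the player and attacks with ranged projectiles, extending a parent enemy class.
; BeginPlay builds a list of four weighted steering behaviors targeting the player.
; Tick drops the fourth behavior when the player is close and restores it when far, with a hysteresis band between.
; Attack fires a BP_Projectile using the Rock data row at the player, scaling damage by a stat from the stat system.
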(event EventBeginPlay
  (bind _steeringbehaviors (Variables|Default|GetSteeringBehaviors))
  (bind _player (Variables|Default|GetPlayer))
  (|CallParentFunction)
  (Utilities|Array|Clear _steeringbehaviors)
  (Utilities|Array|Add _steeringbehaviors (Utilities|Struct|MakeSteeringBehaviorStruct "NewEnumerator5" 0.2 _player 1e+03 5e+02 2e+01 0.0))
  (Utilities|Array|Add _steeringbehaviors (Utilities|Struct|MakeSteeringBehaviorStruct "NewEnumerator1" 0.5 _player 1e+03 2.5e+02 1e+01 7.5e+02))
  (Utilities|Array|Add _steeringbehaviors (Utilities|Struct|MakeSteeringBehaviorStruct "NewEnumerator10" 1.0 _player 5e+02 2.5e+02 1e+01 7.5e+02))
  (Utilities|Array|Add _steeringbehaviors (Utilities|Struct|MakeSteeringBehaviorStruct "NewEnumerator2" 1.0 _player 5e+02 2.5e+02 1e+01 7.5e+02)))

(event EventTick
  (params (DeltaSeconds :type Float%20%28single-precision%29))
  (bind _returnvalue (Transformation|GetActorLocation))
  (bind _steeringbehaviors (Variables|Default|GetSteeringBehaviors))
  (bind _player (Variables|Default|GetPlayer))
  (bind _returnvalue_2 (Transformation|GetActorLocation _player))
  (bind _returnvalue_3 (Math|Vector|Distance(Vector) _returnvalue_2 _returnvalue))
  (|CallParentFunction DeltaSeconds)
  (if (<= _returnvalue_3 1e+03)
    (Utilities|Array|RemoveIndex _steeringbehaviors 3)
    (elif (>= _returnvalue_3 1.5e+03)
      (if (not (Utilities|Array|IsValidIndex _steeringbehaviors 3))
        (Utilities|Array|Add _steeringbehaviors (Utilities|Struct|MakeSteeringBehaviorStruct "NewEnumerator2" 1.0 (Variables|Default|GetPlayer) 5e+02 2.5e+02 1e+01 7.5e+02))))))

(fn ConstructionScript
  (|CallParentFunction))

(fn Attack
  (bind _projectilespawn (Variables|Default|GetProjectileSpawn))
  (bind _returnvalue (Transformation|GetWorldLocation _projectilespawn))
  (|CallParentFunction)
  (Game|SpawnActorfromClass "/Game/Blueprints/Weapons/BP_Projectile.BP_Projectile_C" (Math|Transform|MakeTransform _returnvalue (Math|Rotator|FindLookatRotation _returnvalue (Transformation|GetActorLocation (Variables|Default|GetPlayer))) "1.000000,1.000000,1.000000") "Undefined" "MultiplyWithRoot" 0 "Rock" (+ (* (.Value (Default|GetStat (Variables|Default|GetAC_StatSystem) "NewEnumerator5")) 0.1) 1.0) false 0))