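; BP_Boss is a boss enemy that moves with weighted steering behaviors and reports its defeat when health runs out.
; On BeginPlay it adds three steering behaviors aimed at the player, on top of the parent's setup.
; Attack runs the parent attack, then halts the boss by clearing behaviors and velocity, restoring the same steering after a short delay.
; The stat system's OnZeroHealth event calls CallDefeatedBoss.
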(event OnZeroHealth(AC_StatSystem)
  (Default|CallDefeatedBoss))

(event Custom|AddSteering
  (params (Delay :type Float%20%28double-precision%29))
  (bind _steeringbehaviors (Variables|Default|GetSteeringBehaviors))
  (bind _player (Variables|Default|GetPlayer))
  (Utilities|FlowControl|Delay Delay)
  (Utilities|Array|Add _steeringbehaviors (Utilities|Struct|MakeSteeringBehaviorStruct "NewEnumerator5" 1.0 _player 5e+02 1e+02 2e+01 0.0))
  (Utilities|Array|Add _steeringbehaviors (Utilities|Struct|MakeSteeringBehaviorStruct "NewEnumerator10" 1.0 _player 5e+02 2.5e+02 1e+01 7.5e+02))
  (Utilities|Array|Add _steeringbehaviors (Utilities|Struct|MakeSteeringBehaviorStruct "NewEnumerator2" 1.0 _player 5e+02 2.5e+02 1e+01 7.5e+02)))

(event EventBeginPlay
  (|CallParentFunction)
  (CallFunction|AddSteering 0.0))

(event Collision|EventActorBeginOverlap
  (params (OtherActor :type Actor%20Object%20Reference)))

(event EventTick
  (params (DeltaSeconds :type Float%20%28single-precision%29))
  (|CallParentFunction DeltaSeconds) ; This node is disabled and will not be called.\nDrag off pins to build functionality.
)

(fn ConstructionScript
  (|CallParentFunction))

(fn Attack
  (|CallParentFunction)
  (Utilities|Array|Clear (Variables|Default|GetSteeringBehaviors))
  (Variables|Default|SetVelocity "0, 0, 0")
  (CallFunction|AddSteering 2.0))