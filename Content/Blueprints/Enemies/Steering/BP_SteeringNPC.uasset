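; Steering-behavior NPC actor that moves autonomously using a weighted list of behaviors such as seek, arrive, pursue, wander, spline following, separation and whisker-trace obstacle avoidance.
; Each tick, Locomotion sums CalcSteering results, optionally adjusts vertical steering by ground trace, then integrates clamped force into velocity for swept movement.
; Angular steering drives rotation, with optional facing along velocity.
; Evade, Cohesion and the reached-target handler are empty stubs.
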(event Custom|OnReachedTarge
  (params (SteeringData :type Steering%20Behavior%20Struct%20Structure)))

(event EventBeginPlay
  (EventDispatchers|BindEventtoReachedTarget (delegate Custom|OnReachedTarge))
  (if (Utilities|Array|IsEmpty (Variables|Default|GetSteeringBehaviors))
    _))

(event EventTick
  (params (DeltaSeconds :type Float%20%28single-precision%29))
  (CallFunction|Locomotion)
  (if (Variables|Default|GetAlwaysRotateTowardVelocity)
    (CallFunction|FaceVelocity)))

(fn ConstructionScript
  (|CallParentFunction))

(fn Locomotion
  (Utilities|FlowControl|Sequence
    (:then_0
      (for _array_element (Variables|Default|GetSteeringBehaviors)
        (bind (_steering _steeringangular _islinearsteering) (CallFunction|CalcSteering _array_element))
        (if _islinearsteering
          (LocalVariables|SetTotalSteering (+ (LocalVariables|GetTotalSteering) (* _steering (.Weight (Utilities|Struct|BreakSteeringBehaviorStruct _array_element)))))
          (else
            (LocalVariables|SetTotalSteeringAngular (Math|Rotator|CombineRotators (LocalVariables|GetTotalSteeringAngular) (* _steeringangular (.Weight (Utilities|Struct|BreakSteeringBehaviorStruct _array_element)))))))))
    (:then_1
      (if (Variables|Default|GetUseGroundTrace)
        (bind _outhit (CallFunction|GroundTrace 1e+03))
        ;[0.15 0.15 0.15 0.5] Keep them flat on the ground. Later we can use pathing or line tracing to keep them on the ground even if its elevation changes.
        (if (<= (Variables|Default|GetTargetHeight) (.Distance (Collision|BreakHitResult _outhit)))
          (Variables|Default|SetVelocity (Math|Vector|MakeVector (.x (Variables|Default|GetVelocity)) (.y (Variables|Default|GetVelocity)) (.z (Variables|Default|GetVelocity)))))
        (LocalVariables|SetTotalSteering (* (Math|Vector|Normalize (Math|Vector|MakeVector (.x (LocalVariables|GetTotalSteering)) (.y (LocalVariables|GetTotalSteering)) (Math|Float|SelectFloat (.z (LocalVariables|GetTotalSteering)) (Variables|Default|GetMaxSpeed) (<= (Variables|Default|GetTargetHeight) (.Distance (Collision|BreakHitResult _outhit)))))) (Math|Vector|VectorLength (LocalVariables|GetTotalSteering))))))
    (:then_2
      (LocalVariables|SetSteeringForce (Math|Vector|VectorClampSizeMax (LocalVariables|GetTotalSteering) (Variables|Default|GetMaxAccelLinear))))
    (:then_3
      (LocalVariables|SetAcceleration (/ (LocalVariables|GetSteeringForce) (Variables|Default|GetMass))))
    (:then_4
      (Variables|Default|SetVelocity (Math|Vector|VectorClampSizeMax (+ (Variables|Default|GetVelocity) (LocalVariables|GetAcceleration)) (Variables|Default|GetMaxSpeed))))
    (:then_5
      (Transformation|AddActorWorldOffset (* (Variables|Default|GetVelocity) (Utilities|Time|GetWorldDeltaSeconds)) true))
    (:then_6
      (Class|Actor|AddActorWorldRotation (Math|Rotator|MakeRotator (.roll (* (LocalVariables|GetTotalSteeringAngular) (Utilities|Time|GetWorldDeltaSeconds))) 0.0 (.yaw (* (LocalVariables|GetTotalSteeringAngular) (Utilities|Time|GetWorldDeltaSeconds))))))))

(fn Seek
  (params (TargetPosition :type Vector))
  (return (* (Math|Vector|Normalize (- TargetPosition (CallFunction|GetActorBottom self))) (Variables|Default|GetMaxSpeed))))

(fn Flee
  (params (TargetPosition :type Vector) (Distance :type Float%20%28double-precision%29))
  (bind _returnvalue (Transformation|GetActorLocation))
  (bind _returnvalue_2 (- TargetPosition _returnvalue))
  (if (< (Math|Vector|VectorLength _returnvalue_2) Distance)
    (return (* (Math|Vector|Normalize (* _returnvalue_2 -1.0)) (Variables|Default|GetMaxSpeed)))
    (else
      (return "0, 0, 0"))))

(fn PredictPosition
  (params (TargetLocation :type Vector) (TargetVelocity :type Vector) (MaxPrediction :type Float%20%28double-precision%29))
  (LocalVariables|SetSpeed (Math|Vector|VectorLength (Variables|Default|GetVelocity)))
  (LocalVariables|SetDistance (.Distance (CallFunction|GetVectortoTargetLocation TargetLocation (CallFunction|GetActorBottom self))))
  (bind _output_get (LocalVariables|SetPrediction (select (<= (LocalVariables|GetSpeed) (/ (LocalVariables|GetDistance) MaxPrediction)) MaxPrediction (/ (LocalVariables|GetDistance) (LocalVariables|GetSpeed)))))
  (return (+ TargetLocation (* _output_get TargetVelocity))))

(fn Pursue
  (params (TargetPosition :type Vector) (TargetVelocity :type Vector) (MaxPrediction :type Float%20%28double-precision%29))
  (bind _predictedposition (SteeringBehaviors|PredictPosition TargetPosition TargetVelocity MaxPrediction))
  (CallFunction|QuickDebugArrow _predictedposition "(R=0.000000,G=1.000000,B=0.000000,A=1.000000)" 0.0)
  (return (SteeringBehaviors|Arrive 0.0 5e+01 0.1 _predictedposition)))

(fn CalcSteering
  (params (SteeringData :type Steering%20Behavior%20Struct%20Structure))
  (bind _target (Utilities|Struct|BreakSteeringBehaviorStruct SteeringData))
  (bind _target_2 (Utilities|Struct|BreakSteeringBehaviorStruct SteeringData))
  (bind _target_3 (Utilities|Struct|BreakSteeringBehaviorStruct SteeringData))
  (bind (_type _weight _target_4 _fleedistance _wanderradius _wanderrate _wanderoffset) (Utilities|Struct|BreakSteeringBehaviorStruct SteeringData))
  (bind (_type_2 _weight_2 _target_5 _fleedistance_2) (Utilities|Struct|BreakSteeringBehaviorStruct SteeringData))
  (switch Utilities|FlowControl|Switch|SwitchonSteeringBehaviorType (.type SteeringData)
    (:NewEnumerator0
      (return (SteeringBehaviors|Seek (Transformation|GetActorLocation (.Target (Utilities|Struct|BreakSteeringBehaviorStruct SteeringData)))) "0, 0, 0" true))
    (:NewEnumerator1
      (return (SteeringBehaviors|Flee (Transformation|GetActorLocation _target_5) _fleedistance_2) "0, 0, 0" true))
    (:NewEnumerator2
      (return (SteeringBehaviors|Arrive 3e+02 7.5e+02 1.0 (Transformation|GetActorLocation (.Target (Utilities|Struct|BreakSteeringBehaviorStruct SteeringData)))) "0, 0, 0" true))
    (:NewEnumerator3
      (Utilities|IsValid _target_2
        (:Is%20Valid
          (bind _asbp_steering_npc (Utilities|Casting|CastToBP_SteeringNPC _target_2))
          (return (SteeringBehaviors|Pursue (CallFunction|GetActorBottom) (Variables|BP_SteeringNPC_C|GetVelocity _asbp_steering_npc) 5e+01) "0, 0, 0" true))))
    (:NewEnumerator4
      (Utilities|IsValid _target_3
        (:Is%20Valid
          (bind _asbp_steering_npc_2 (Utilities|Casting|CastToBP_SteeringNPC _target_3))
          (return (SteeringBehaviors|Evade (CallFunction|GetActorBottom) (Variables|BP_SteeringNPC_C|GetVelocity _asbp_steering_npc_2) 5e+02) "0, 0, 0" true))))
    (:NewEnumerator5
      (bind _steering (SteeringBehaviors|Wander _wanderradius _wanderrate _wanderoffset))
      (return _steering "0, 0, 0" true))
    (:NewEnumerator6
      (bind _steering_2 (SteeringBehaviors|PathFollowingSimple SteeringData 2e+02))
      (return _steering_2 "0, 0, 0" true))
    (:NewEnumerator7
      (bind _steering_3 (SteeringBehaviors|ObstacleAvoidance))
      (return _steering_3 "0, 0, 0" true))
    (:NewEnumerator8
      (Utilities|IsValid _target
        (:Is%20Valid
          (bind _asbp_steering_npc_3 (Utilities|Casting|CastToBP_SteeringNPC _target))
          (bind _steering_4 (SteeringBehaviors|VelocityMatching 0.1 (Variables|BP_SteeringNPC_C|GetVelocity _asbp_steering_npc_3)))
          (return _steering_4 "0, 0, 0" true))))
    (:NewEnumerator9
      (bind _steeringangular (SteeringBehaviors|Align2D SteeringData 0.0 2e+01 0.1))
      (return "0, 0, 0" _steeringangular false))
    (:NewEnumerator10
      (return (SteeringBehaviors|Fly (Transformation|GetActorLocation (.target SteeringData)) (Variables|Default|GetTargetHeight)) "0, 0, 0" true))
    (:NewEnumerator11
      (bind _neighbors (CallFunction|FindNeighbors (Variables|Default|GetNeighborRadius)))
      (bind _steering_5 (SteeringBehaviors|Separation _neighbors 5e+02))
      (return _steering_5 "0, 0, 0" true))))

(fn Wander
  (params (WanderRadius :type Float%20%28double-precision%29) (WanderRate :type Float%20%28double-precision%29) (WanderOffset :type Float%20%28double-precision%29))
  (bind _returnvalue (Transformation|GetActorForwardVector))
  (bind _output_get (Variables|Default|SetWanderRandomDegrees (+ (Variables|Default|GetWanderRandomDegrees) (* WanderRate (- (Math|Random|RandomFloat) (Math|Random|RandomFloat))))))
  (return (SteeringBehaviors|Seek (+ (+ (CallFunction|GetActorBottom self) (* _returnvalue WanderOffset)) (* (Math|Vector|RotateVectorAroundAxis _returnvalue (Variables|Default|GetWanderRandomDegrees) (Transformation|GetActorUpVector)) WanderRadius)))))

(fn Arrive
  (params (TargetRadius :type Float%20%28double-precision%29) (SlowingRadius :type Float%20%28double-precision%29) (TimeToTarget :type Float%20%28double-precision%29) (Target :type Vector))
  (bind _self self)
  (bind _returnvalue (Transformation|GetActorLocation _self))
  (bind _returnvalue_2 (- Target _returnvalue))
  (bind _returnvalue_3 (Math|Vector|VectorLength _returnvalue_2))
  (if (<= _returnvalue_3 TargetRadius)
    (return "0, 0, 0")
    (else
      (return (/ (- (* (Math|Vector|Normalize _returnvalue_2) (Math|Float|SelectFloat (Variables|Default|GetMaxSpeed) (/ (* _returnvalue_3 (Variables|Default|GetMaxSpeed)) SlowingRadius) (> _returnvalue_3 SlowingRadius))) (Variables|Default|GetVelocity)) TimeToTarget)))))

(fn FaceVelocity
  (bind _velocity (Variables|Default|GetVelocity))
  (bind _returnvalue (Math|Rotator|MakeRotfromX _velocity))
  (if (>= (Math|Vector|VectorLengthSquared _velocity) 25.0)
    (Transformation|SetActorRotation (Math|Rotator|MakeRotator (.roll _returnvalue) 0.0 (.yaw _returnvalue)))))

(fn VelocityMatching
  (params (TimeToTarget :type Float%20%28double-precision%29) (TargetVelocity :type Vector))
  (return (Math|Vector|VectorClampSizeMax (/ (- TargetVelocity (Variables|Default|GetVelocity)) TimeToTarget) (Variables|Default|GetMaxAccelLinear))))

(fn Evade
  (params (TargetLocation :type Vector) (TargetVelocity :type Vector) (MaxPrediction :type Float%20%28double-precision%29)))

(fn ObstacleAvoidanceWhisker
  (params (Direction :type Vector) (Length :type Float%20%28double-precision%29) (AvoidanceOffset :type Float%20%28double-precision%29))
  (bind _returnvalue (Transformation|GetActorLocation))
  (bind _outhit (Collision|LineTraceByChannel _returnvalue (+ _returnvalue (* Direction Length)) "TraceTypeQuery1" false 0 "ForOneFrame"))
  (if (.bBlockingHit (Collision|BreakHitResult _outhit))
    (return (SteeringBehaviors|Seek (+ (.Location (Collision|BreakHitResult _outhit)) (* (.Normal (Collision|BreakHitResult _outhit)) AvoidanceOffset))))
    (else
      (return "0, 0, 0"))))

(fn ObstacleAvoidance
  (Utilities|FlowControl|Sequence
    (:then_0
      (Utilities|FlowControl|Sequence
        (:then_0
          (bind _steering (SteeringBehaviors|ObstacleAvoidanceWhisker (Transformation|GetActorForwardVector) 5e+02 5e+02))
          (LocalVariables|SetTotal (+ (LocalVariables|GetTotal) _steering)))
        (:then_1
          (bind _steering_2 (SteeringBehaviors|ObstacleAvoidanceWhisker (Math|Vector|RotateVectorAroundAxis (Transformation|GetActorForwardVector) -3e+01 "0.000000,0.000000,1.000000") 3e+02 4e+02))
          (LocalVariables|SetTotal (+ (LocalVariables|GetTotal) _steering_2)))
        (:then_2
          (bind _steering_3 (SteeringBehaviors|ObstacleAvoidanceWhisker (Math|Vector|RotateVectorAroundAxis (Transformation|GetActorForwardVector) 3e+01 "0.000000,0.000000,1.000000") 3e+02 4e+02))
          (LocalVariables|SetTotal (+ (LocalVariables|GetTotal) _steering_3)))))
    (:then_1
      (return (LocalVariables|GetTotal)))))

(fn PathFollowingSimple
  (params (SteeringData :type Steering%20Behavior%20Struct%20Structure) (PathOffset :type Float%20%28double-precision%29))
  (bind _returnvalue (Actor|GetComponentbyClass (.target SteeringData) "/Script/Engine.SplineComponent"))
  (bind _returnvalue_2 (Transformation|GetActorLocation))
  (bind _returnvalue_3 (Class|SplineComponent|GetDistanceAlongSplineatLocation _returnvalue _returnvalue_2 "World"))
  (bind _returnvalue_4 (+ _returnvalue_3 PathOffset))
  (bind _returnvalue_5 (Spline|GetLocationatDistanceAlongSpline _returnvalue _returnvalue_4 "World"))
  (Utilities|IsValid _returnvalue
    (:Is%20Valid
      (Rendering|Debug|DrawDebugPoint (Spline|GetLocationatDistanceAlongSpline _returnvalue _returnvalue_3 "World") 1e+01 "(R=1.000000,G=0.076232,B=0.000000,A=1.000000)" 0.0)
      (Rendering|Debug|DrawDebugPoint _returnvalue_5 1e+01 "(R=0.000000,G=0.078744,B=1.000000,A=1.000000)" 0.0)
      (return (SteeringBehaviors|Seek _returnvalue_5)))
    (:Is%20Not%20Valid
      (return "0, 0, 0"))))

(fn PathFollowingPredictive
  (params (SteeringData :type Steering%20Behavior%20Struct%20Structure) (PredictionTime :type Float%20%28double-precision%29) (PathOffset :type Float%20%28double-precision%29))
  (bind _returnvalue (Actor|GetComponentbyClass (.target SteeringData) "/Script/Engine.SplineComponent"))
  (bind _self self)
  (bind _velocity (Variables|Default|GetVelocity))
  (bind _returnvalue_2 (CallFunction|GetActorBottom _self))
  (bind _returnvalue_3 (* _velocity PredictionTime))
  (bind _returnvalue_4 (+ _returnvalue_2 _returnvalue_3))
  (bind _returnvalue_5 (Class|SplineComponent|GetDistanceAlongSplineatLocation _returnvalue _returnvalue_4 "World"))
  (bind _returnvalue_6 (+ _returnvalue_5 PathOffset))
  (bind _returnvalue_7 (Spline|GetLocationatDistanceAlongSpline _returnvalue _returnvalue_6 "World"))
  (Utilities|IsValid _returnvalue
    (:Is%20Valid
      (Rendering|Debug|DrawDebugPoint (Spline|GetLocationatDistanceAlongSpline _returnvalue _returnvalue_5 "World") 1e+01 "(R=1.000000,G=0.076232,B=0.000000,A=1.000000)" 0.0)
      (Rendering|Debug|DrawDebugPoint _returnvalue_7 1e+01 "(R=0.000000,G=0.078744,B=1.000000,A=1.000000)" 0.0)
      (return (SteeringBehaviors|Seek _returnvalue_7)))
    (:Is%20Not%20Valid
      (return "0, 0, 0"))))

(fn Align2D
  (params (Steering%20Data :type Steering%20Behavior%20Struct%20Structure) (TargetRotationDelta :type Float%20%28double-precision%29) (SlowRotationDelta :type Float%20%28double-precision%29) (TimeToTarget :type Float%20%28double-precision%29))
  (bind _returnvalue (Transformation|GetActorRotation))
  (bind _returnvalue_2 (Transformation|GetActorRotation (.target Steering%20Data)))
  (bind _maxrotation (Variables|Default|GetMaxRotation))
  (bind _maxaccelangular (Variables|Default|GetMaxAccelAngular))
  (bind _returnvalue_3 (Math|Rotator|Delta(Rotator) _returnvalue_2 _returnvalue))
  (bind _yaw (Math|Rotator|BreakRotator _returnvalue_3))
  (LocalVariables|SetrotationDelta _yaw)
  (bind _output_get (LocalVariables|SetrotationMagnitude (Math|Float|Absolute(Float) _yaw)))
  (if (< _output_get TargetRotationDelta)
    (return "0, 0, 0")
    (else
      (bind _output_get_2 (LocalVariables|SettargetRotation (select (> (LocalVariables|GetrotationMagnitude) SlowRotationDelta) _maxrotation (/ (* _maxrotation (LocalVariables|GetrotationMagnitude)) SlowRotationDelta))))
      (bind _output_get_3 (LocalVariables|SettargetRotation (* _output_get_2 (/ (LocalVariables|GetrotationDelta) (LocalVariables|GetrotationMagnitude)))))
      (bind _output_get_4 (LocalVariables|SetresultRotation (/ (- _output_get_3 (Class|KismetMathLibrary|VectorCosineAngle2D (Transformation|GetActorForwardVector) "1.000000,0.000000,0.000000")) TimeToTarget)))
      (if (> (Math|Float|Absolute(Float) _output_get_4) _maxaccelangular)
        (bind _output_get_5 (LocalVariables|SetresultRotation (* _maxaccelangular (/ (LocalVariables|GetresultRotation) (Math|Float|Absolute(Float) _output_get_4))))))
      (return (Math|Rotator|MakeRotator 0.0 0.0 _output_get_5)))))

(fn Cohesion
  (params (CenterOfNeighbors :type Vector)))

(fn Separation
  (params (Neighbors :type Array%20of%20Actor%20Object%20References) (DistanceThreshold :type Float%20%28double-precision%29))
  (for _array_element Neighbors
    (if (< (.Distance (CallFunction|GetVectortoTargetLocation (Transformation|GetActorLocation _array_element) (Transformation|GetActorLocation))) DistanceThreshold)
      (bind _output_get (LocalVariables|SetRepelStrength (/ (* (- DistanceThreshold (.Distance (CallFunction|GetVectortoTargetLocation (Transformation|GetActorLocation _array_element) (Transformation|GetActorLocation)))) (Variables|Default|GetMaxAccelLinear)) DistanceThreshold)))
      (LocalVariables|SetResult (+ (LocalVariables|GetResult) (* _output_get (.Direction (CallFunction|GetVectortoTargetLocation (Transformation|GetActorLocation _array_element) (Transformation|GetActorLocation))) -1.0)))))
  (return (LocalVariables|GetResult)))

(fn GroundTrace
  (params (Distance :type Float%20%28double-precision%29))
  (bind _self self)
  (bind _returnvalue (CallFunction|GetActorBottom _self))
  (bind (_x _y _z) (Math|Vector|BreakVector _returnvalue))
  (bind (_outhit _returnvalue_2) (Collision|LineTraceByChannel _returnvalue (Math|Vector|MakeVector _x _y (* (* _z Distance) -1.0)) "TraceTypeQuery1" false 0 "None"))
  (return _outhit _returnvalue_2))

(fn Fly
  (params (TargetPosition :type Vector) (TargetHeight :type Float%20%28double-precision%29))
  (return (Math|Vector|MakeVector 0.0 0.0 (.z (* (Math|Vector|Normalize (- (Math|Vector|MakeVector (.x TargetPosition) (.y TargetPosition) (+ (.z TargetPosition) TargetHeight)) (CallFunction|GetActorBottom self))) (Variables|Default|GetMaxSpeed))))))