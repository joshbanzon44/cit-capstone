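; Blueprint function library of shared math, movement and debug helpers for enemy steering.
; GoToTarget turns an actor toward a target actor or fallback location and moves it there at frame-scaled speed without sweeping, measuring from its bounds bottom and returning the distance.
; Other helpers provide a random binomial value, evenly spaced points on a horizontal circle (the degree offset input is unused) and a downward debug arrow.
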(fn GetVectortoTargetLocation
  (params (TargetLocation :type Vector) (OriginLocation :type Vector))
  (bind _returnvalue (- TargetLocation OriginLocation))
  (return (Math|Vector|VectorLength _returnvalue) (Math|Vector|Normalize _returnvalue) _returnvalue))

(fn PerFrameSpeed
  (params (CMPerSecond :type Float%20%28double-precision%29) (DeltaTime :type Float%20%28double-precision%29))
  (return (* CMPerSecond DeltaTime)))

(fn GetActorBottom
  (params (Actor :type Actor%20Object%20Reference))
  (bind (_origin _boxextent) (Collision|GetActorBounds Actor false false))
  (Utilities|IsValid Actor
    (:Is%20Valid
      (return (- _origin (Math|Vector|MakeVector 0.0 0.0 (.Z (Math|Vector|BreakVector _boxextent))))))))

(fn RandomBinomial
  (return (- (Math|Random|RandomFloat) (Math|Random|RandomFloat))))

(fn GotoTarget
  (params (Actor :type Actor%20Object%20Reference) (TargetActor :type Actor%20Object%20Reference) (TargetLocation :type Vector) (MaxSpeed :type Float%20%28double-precision%29))
  (Utilities|IsValid TargetActor
    (:Is%20Valid
      (LocalVariables|SetFinalTarget (Transformation|GetActorLocation TargetActor)))
    (:Is%20Not%20Valid
      (LocalVariables|SetFinalTarget TargetLocation)))
  (Transformation|SetActorRotation Actor (Math|Rotator|MakeRotfromX (* (CallFunction|PerFrameSpeed MaxSpeed (Utilities|Time|GetWorldDeltaSeconds)) (.Direction (CallFunction|GetVectortoTargetLocation (LocalVariables|GetFinalTarget) (CallFunction|GetActorBottom Actor))))))
  (Transformation|AddActorWorldOffset Actor (* (CallFunction|PerFrameSpeed MaxSpeed (Utilities|Time|GetWorldDeltaSeconds)) (.Direction (CallFunction|GetVectortoTargetLocation (LocalVariables|GetFinalTarget) (CallFunction|GetActorBottom Actor)))))
  (return (.Distance (CallFunction|GetVectortoTargetLocation (LocalVariables|GetFinalTarget) (CallFunction|GetActorBottom Actor)))))

(fn QuickDebugArrow
  (params (Location :type Vector) (Color :type Linear%20Color%20Structure :default "(R=0.000000,G=1.000000,B=0.000000,A=1.000000)") (Duration :type Float%20%28single-precision%29))
  (Rendering|Debug|DrawDebugArrow 0 (+ Location "0.000000,0.000000,100.000000") Location 1.5e+02 Color Duration 1e+01))

(fn GetPointsinCircle
  (params (Radius :type Float%20%28double-precision%29) (Number :type Integer) (OffsetDegrees :type Float%20%28double-precision%29))
  (Utilities|Array|Resize (LocalVariables|GetResult) Number)
  (for _index (range 0 Number)
    (Utilities|Array|SetArrayElem (LocalVariables|GetResult) _index (Math|Vector|RotateVectorAroundAxis (Math|Vector|MakeVector Radius 0.0 0.0) (* _index (/ 360 (Math|Conversions|ToFloat(Integer) Number))) "0.000000,0.000000,1.000000")))
  (return (LocalVariables|GetResult)))