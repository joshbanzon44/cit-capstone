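; Actor component that stores character stats in a map and handles health limits and leveling.
; Get, set, add and subtract functions update the map and fire change dispatchers, with add and subtract running Health, Defense and Exp checks.
; Level-up carries surplus Exp, adds DT_LevelStatsPlayer row gains (falling back to "Max"), refills Health and rechecks recursively.
; A table lookup by OwnerType is unconnected, so leveling always uses the player table.
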(event Custom|CheckMaxExp
  (bind _value (CallFunction|GetStat "NewEnumerator7"))
  (if (>= (.Value (CallFunction|GetStat "NewEnumerator1")) _value)
    (Default|CallOnLevelUp)
    (CallFunction|SubtractStatValue "NewEnumerator1" _value)
    (CallFunction|AddStatValue "NewEnumerator0" 1.0)
    (bind _returnvalue (Utilities|GetDataTableRow "/Game/DataTables/LevelUpStats/DT_LevelStatsPlayer.DT_LevelStatsPlayer" (Utilities|String|StringToName (Utilities|String|ToString(Integer) (Class|KismetMathLibrary|ToInt64(Float) (.Value (CallFunction|GetStat "NewEnumerator0"))))))
      (:then
        (CallFunction|AddStatValue "NewEnumerator7" (.maxexp _returnvalue))
        (CallFunction|AddStatValue "NewEnumerator3" (.maxhealth _returnvalue))
        (CallFunction|AddStatValue "NewEnumerator4" (.speed _returnvalue))
        (CallFunction|AddStatValue "NewEnumerator5" (.strength _returnvalue))
        (CallFunction|AddStatValue "NewEnumerator6" (.defense _returnvalue))
        (CallFunction|AddStatValue "NewEnumerator9" (.atkspeed _returnvalue)))
      (:RowNotFound
        (bind _returnvalue_2 (Utilities|GetDataTableRow "/Game/DataTables/LevelUpStats/DT_LevelStatsPlayer.DT_LevelStatsPlayer" "Max")
          (:then
            (CallFunction|AddStatValue "NewEnumerator7" (.maxexp _returnvalue_2))
            (CallFunction|AddStatValue "NewEnumerator3" (.maxhealth _returnvalue_2))
            (CallFunction|AddStatValue "NewEnumerator4" (.speed _returnvalue_2))
            (CallFunction|AddStatValue "NewEnumerator5" (.strength _returnvalue_2))
            (CallFunction|AddStatValue "NewEnumerator6" (.defense _returnvalue_2))
            (CallFunction|AddStatValue "NewEnumerator9" (.atkspeed _returnvalue_2))))))
    (CallFunction|SetStatValue "NewEnumerator2" (.Value (CallFunction|GetStat "NewEnumerator3")))
    (CallFunction|CheckMaxExp)))

(event Custom|CheckMaxDefense
  (if (> (.Value (CallFunction|GetStat "NewEnumerator6")) 1e+02)
    (CallFunction|SetStatValue "NewEnumerator6" 1e+02)))

(event Custom|CheckMaxHealth
  (bind _value (CallFunction|GetStat "NewEnumerator3"))
  (if (> (.Value (CallFunction|GetStat "NewEnumerator2")) _value)
    (CallFunction|SetStatValue "NewEnumerator2" _value)))

(event Custom|CheckMinHealth
  (if (<= (.Value (CallFunction|GetStat "NewEnumerator2")) 0.0)
    (Default|CallOnZeroHealth)))

(event EventBeginPlay
  (Default|CallOnHUDStatChange))

(fn GetStat
  (params (Key :type Enum_Stats%20Enum :default "NewEnumerator0"))
  (bind _stats (Variables|Default|GetStats))
  (bind (_value _returnvalue) (Utilities|Map|Find _stats Key))
  (return _value _returnvalue))

(fn SetStatValue
  (params (SelectStat :type Enum_Stats%20Enum :default "NewEnumerator0") (SetValue :type Float%20%28double-precision%29))
  (Utilities|Map|Add (Variables|Default|GetStats) SelectStat SetValue)
  (switch Utilities|FlowControl|Switch|SwitchonEnum_Stats SelectStat
    (:NewEnumerator8
      _)
    (:NewEnumerator0
      _)
    (:NewEnumerator1
      _)
    (:NewEnumerator7
      _)
    (:NewEnumerator2
      _)
    (:NewEnumerator3
      _)
    (:NewEnumerator12
      _)
    (:NewEnumerator4
      _)
    (:NewEnumerator10
      _)
    (:NewEnumerator5
      _)
    (:NewEnumerator6
      _)
    (:NewEnumerator9
      _)
    (:NewEnumerator13
      _))
  (Default|CallOnHUDStatChange)
  (Default|CallOnAnyStatChange)
  (return (.Value (CallFunction|GetStat SelectStat))))

(fn AddStatValue
  (params (SelectStat :type Enum_Stats%20Enum :default "NewEnumerator0") (AddValue :type Float%20%28double-precision%29))
  (Utilities|Map|Add (Variables|Default|GetStats) SelectStat (+ AddValue (.Value (CallFunction|GetStat SelectStat))))
  (switch Utilities|FlowControl|Switch|SwitchonEnum_Stats SelectStat
    (:NewEnumerator8
      _)
    (:NewEnumerator0
      _)
    (:NewEnumerator1
      (CallFunction|CheckMaxExp)
      (Default|CallOnHUDStatChange :!label _label))
    (:NewEnumerator7
      _)
    (:NewEnumerator2
      (CallFunction|CheckMaxHealth)
      (goto _label))
    (:NewEnumerator3
      _)
    (:NewEnumerator12
      _)
    (:NewEnumerator4
      _)
    (:NewEnumerator10
      _)
    (:NewEnumerator5
      _)
    (:NewEnumerator6
      (CallFunction|CheckMaxDefense)
      (goto _label))
    (:NewEnumerator9
      _)
    (:NewEnumerator11
      _)
    (:NewEnumerator13
      _))
  (Default|CallOnAnyStatChange)
  (return (.Value (CallFunction|GetStat SelectStat))))

(fn SubtractStatValue
  (params (SelectStat :type Enum_Stats%20Enum :default "NewEnumerator0") (SubtractValue :type Float%20%28double-precision%29))
  (Utilities|Map|Add (Variables|Default|GetStats) SelectStat (- (.Value (CallFunction|GetStat SelectStat)) SubtractValue))
  (switch Utilities|FlowControl|Switch|SwitchonEnum_Stats SelectStat
    (:NewEnumerator8
      _)
    (:NewEnumerator0
      _)
    (:NewEnumerator1
      _)
    (:NewEnumerator7
      _)
    (:NewEnumerator2
      (CallFunction|CheckMinHealth)
      (Default|CallOnHUDStatChange))
    (:NewEnumerator3
      _)
    (:NewEnumerator12
      _)
    (:NewEnumerator4
      _)
    (:NewEnumerator10
      _)
    (:NewEnumerator5
      _)
    (:NewEnumerator6
      _)
    (:NewEnumerator9
      _)
    (:NewEnumerator13
      _))
  (Default|CallOnAnyStatChange)
  (return (.Value (CallFunction|GetStat SelectStat))))