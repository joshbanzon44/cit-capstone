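; Frost effect actor that spins a Niagara effect and damages enemies inside its sphere.
; A restarting Timeline drives the effect's world yaw from BeginPlay, while Tick sends Damage to every overlapping BP_Base_Enemy each frame, unscaled by delta time.
; ActivateFunc and DectivateFunc toggle the Niagara effect and actor tick together, with a debug print on activation.
; Despite the name, the Spline goes unused in the graphs.
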(event EventBeginPlay
  (bind _newtrack_0 (Timeline|Timeline PlayFromStart)
    (:Update
      (Transformation|SetWorldRotation (Variables|Default|GetNiagara) (Math|Rotator|MakeRotator 0.0 0.0 _newtrack_0) false false))
    (:Finished
      (Timeline|Timeline PlayFromStart))))

(event Collision|EventActorBeginOverlap
  (params (OtherActor :type Actor%20Object%20Reference)))

(event EventTick
  (params (DeltaSeconds :type Float%20%28single-precision%29))
  (for _array_element (Collision|GetOverlappingActors (Variables|Default|GetSphere) "/Game/Blueprints/Enemies/BP_Base_Enemy.BP_Base_Enemy_C" :!class /Script/Engine.PrimitiveComponent)
    (Class|BPDamagable|TakeDamage(Message) _array_element (Variables|Default|GetDamage))))

(fn ConstructionScript)

(fn ActivateFunc
  (Components|Activation|Activate (Variables|Default|GetNiagara) true)
  (Actor|Tick|SetActorTickEnabled true)
  (Development|PrintString (Utilities|String|ToString(Boolean) (Components|Activation|IsActive (Variables|Default|GetNiagara)))))

(fn DectivateFunc
  (Components|Activation|Deactivate (Variables|Default|GetNiagara))
  (Actor|Tick|SetActorTickEnabled false))