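; Base component for the player's timed active abilities, configured from a row in DT_Ability_Active.
; BeginPlay caches the row data, attaches an inactive Niagara system to the player's mesh socket and spawns an optional bound actor there.
; Activation toggles the frost spline actor, or otherwise the Niagara effect and tick, then ends after Duration.
; Healing Aura and Ammo Amplifier stat effects are hardcoded by ability name; StopAbility destroys the spawned visuals.
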(event Custom|StopAbility
  (bind _niagraracomponent (Variables|Default|GetNiagraraComponent))
  (bind _attachedactor (Variables|Default|GetAttachedActor))
  (Utilities|IsValid _attachedactor
    (:Is%20Valid
      (Actor|DestroyActor _attachedactor))
    (:Is%20Not%20Valid
      _))
  (Utilities|IsValid _niagraracomponent
    (:Is%20Valid
      (Components|DestroyComponent _niagraracomponent))))

(event Custom|ActivateAbility
  (bind _asbp_spline_vfx_frost (Utilities|Casting|CastToBP_SplineVFX_Frost (Variables|Default|GetAttachedActor))
    (:then
      (Default|ActivateFunc _asbp_spline_vfx_frost)
      (Development|PrintString "activate"))
    (:CastFailed
      (Components|Activation|Activate (Variables|Default|GetNiagraraComponent) false)
      (Components|Tick|SetComponentTickEnabled true)
      (if (== (Variables|Default|GetAbilityName) "Ammo Amplifier")
        (Default|AddStatValue (Variables|/Game/Blueprints/BP_Player.BP_Player_C|GetAC_StatSystem (Variables|Default|GetPlayer)) "NewEnumerator9" 5e+01))))
  (Utilities|FlowControl|Delay (Variables|Default|GetDuration))
  (CallFunction|EndUse))

(event Custom|EndUse
  (bind _asbp_spline_vfx_frost (Utilities|Casting|CastToBP_SplineVFX_Frost (Variables|Default|GetAttachedActor))
    (:then
      (Default|DectivateFunc _asbp_spline_vfx_frost))
    (:CastFailed
      (Components|Activation|Deactivate (Variables|Default|GetNiagraraComponent))
      (Components|Tick|SetComponentTickEnabled false)
      (if (== (Variables|Default|GetAbilityName) "Ammo Amplifier")
        (Default|SubtractStatValue (Variables|/Game/Blueprints/BP_Player.BP_Player_C|GetAC_StatSystem (Variables|Default|GetPlayer)) "NewEnumerator9" 5e+01)))))

(event EventBeginPlay
  (bind _returnvalue (Utilities|GetDataTableRow "/Game/DataTables/DT_Ability_Active.DT_Ability_Active" (Variables|Default|GetDT_RowName))
    (:then
      (Variables|Default|SetAbilityName (.name _returnvalue))
      (Variables|Default|SetIcon (.icon _returnvalue))
      (Variables|Default|SetCooldown (.cooldown _returnvalue))
      (Variables|Default|SetDuration (.duration _returnvalue))
      (bind _output_get (Variables|Default|SetNiagaraSystem (.particlesystem _returnvalue)))
      (bind _asbp_player (Utilities|Casting|CastToBP_Player (Components|GetOwner)))
      (bind _output_get_2 (Variables|Default|SetPlayer _asbp_player))
      (bind _output_get_3 (Variables|Default|SetSocket (.socket _returnvalue)))
      (bind _returnvalue_2 (Niagara|SpawnSystemAttached _output_get (Variables|/Script/Engine.Character|GetMesh _output_get_2) _output_get_3 "0, 0, 0" "0, 0, 0" "KeepRelativeOffset" false false))
      (Variables|Default|SetNiagraraComponent _returnvalue_2)
      (Variables|Default|SetActorToBind (.actortobind _returnvalue))
      (bind _returnvalue_3 (Game|SpawnActorfromClass (Variables|Default|GetActorToBind) (Math|Transform|MakeTransform (Transformation|GetActorLocation (Variables|Default|GetPlayer)) "0, 0, 0" "1.000000,1.000000,1.000000") "Undefined" "MultiplyWithRoot" 0 0))
      (bind _output_get_4 (Variables|Default|SetAttachedActor _returnvalue_3))
      (Utilities|IsValid _output_get_4
        (:Is%20Valid
          (Transformation|AttachComponentToComponent _output_get_4 (Variables|/Script/Engine.Character|GetMesh (Variables|Default|GetPlayer)) (Variables|Default|GetSocket) "SnapToTarget" "KeepWorld" "KeepRelative" true))))))

(event EventTick
  (params (DeltaSeconds :type Float%20%28single-precision%29))
  (bind _player (Variables|Default|GetPlayer))
  (bind _ac_statsystem (Variables|/Game/Blueprints/BP_Player.BP_Player_C|GetAC_StatSystem _player))
  (if (== (Variables|Default|GetAbilityName) "Healing Aura")
    (Default|AddStatValue _ac_statsystem "NewEnumerator2" (* (.Value (Default|GetStat _ac_statsystem "NewEnumerator3")) 0.05))
    (Development|PrintString "add health")))