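; Ability manager component that gives its owner passive and active abilities, each as its own component configured by a data table row name.
; On BeginPlay it creates components from the Abilities list, capped per type by a max amount.
; OnNewAbilityItem appends a new ability, or once that type holds two (hard-coded), destroys the named old component through a player or enemy cast and inserts the replacement at its index.
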(event Custom|OnNewAbilityItem
  (params (NewName :type Name) (OldName :type Name) (IsPassive :type Boolean))
  (bind _returnvalue (Components|GetOwner))
  (bind _returnvalue_2 (Components|GetOwner))
  (bind _returnvalue_3 (Components|GetOwner))
  (if IsPassive
    (if (>= (Utilities|Array|Length (Variables|Default|GetAC_PassiveAbilities)) 2)
      (for (_array_element _array_index) (Variables|Default|GetAC_PassiveAbilities)
        (if (== (Variables|/Game/Blueprints/Components/Abilities/AC_Base_PassiveAbility.AC_Base_PassiveAbility_C|GetDT_RowName _array_element) OldName)
          (Variables|Default|SetPassiveIndexToRemove _array_index)
          (bind _asbp_player (Utilities|Casting|CastToBP_Player _returnvalue_3)
            (:then
              (Default|DestroyOwnedComponent _asbp_player _array_element)
              (Utilities|Array|RemoveItem (Variables|Default|GetAC_PassiveAbilities) _array_element))
            (:CastFailed
              (bind _asbp_base_enemy (Utilities|Casting|CastToBP_Base_Enemy _returnvalue_3))
              (Default|DestroyOwnedComponent _asbp_base_enemy _array_element)))))
      (bind _returnvalue_4 (Game|AddComponentbyClass _returnvalue "/Game/Blueprints/Components/Abilities/AC_Base_PassiveAbility.AC_Base_PassiveAbility_C" NewName))
      (Utilities|Array|Insert (Variables|Default|GetAC_PassiveAbilities) _returnvalue_4 (Variables|Default|GetPassiveIndexToRemove))
      (else
        (bind _returnvalue_5 (Game|AddComponentbyClass (Components|GetOwner) "/Game/Blueprints/Components/Abilities/AC_Base_PassiveAbility.AC_Base_PassiveAbility_C" NewName))
        (Utilities|Array|Add (Variables|Default|GetAC_PassiveAbilities) _returnvalue_5)))
    (elif (>= (Utilities|Array|Length (Variables|Default|GetAC_ActiveAbilities)) 2)
      (for (_array_element_2 _array_index_2) (Variables|Default|GetAC_ActiveAbilities)
        (if (== (Variables|/Game/Blueprints/Components/Abilities/AC_Base_ActiveAbiltiy.AC_Base_ActiveAbiltiy_C|GetDT_RowName _array_element_2) OldName)
          (Variables|Default|SetActiveIndexToRemove _array_index_2)
          (bind _asbp_player_2 (Utilities|Casting|CastToBP_Player _returnvalue_2)
            (:then
              (Default|DestroyOwnedComponent _asbp_player_2 _array_element_2))
            (:CastFailed
              (bind _asbp_base_enemy_2 (Utilities|Casting|CastToBP_Base_Enemy _returnvalue_2))
              (Default|DestroyOwnedComponent _asbp_base_enemy_2 _array_element_2)))
          (Utilities|Array|RemoveItem (Variables|Default|GetAC_ActiveAbilities) _array_element_2)))
      (bind _returnvalue_6 (Game|AddComponentbyClass _returnvalue "/Game/Blueprints/Components/Abilities/AC_Base_ActiveAbiltiy.AC_Base_ActiveAbiltiy_C" NewName))
      (Utilities|Array|Insert (Variables|Default|GetAC_ActiveAbilities) _returnvalue_6 (Variables|Default|GetActiveIndexToRemove))
      (else
        (bind _returnvalue_7 (Game|AddComponentbyClass (Components|GetOwner) "/Game/Blueprints/Components/Abilities/AC_Base_ActiveAbiltiy.AC_Base_ActiveAbiltiy_C" NewName))
        (Utilities|Array|Add (Variables|Default|GetAC_ActiveAbilities) _returnvalue_7)))))

(event EventBeginPlay
  (bind _returnvalue (Components|GetOwner))
  (for _array_element (Variables|Default|GetAbilities)
    (if (.ispassive _array_element)
      (if (not (>= (Utilities|Array|Length (Variables|Default|GetAC_PassiveAbilities)) (Variables|Default|GetMaxPassiveAmt)))
        (bind _returnvalue_2 (Game|AddComponentbyClass _returnvalue "/Game/Blueprints/Components/Abilities/AC_Base_PassiveAbility.AC_Base_PassiveAbility_C" (.name _array_element)))
        (Utilities|Array|Add (Variables|Default|GetAC_PassiveAbilities) _returnvalue_2))
      (elif (not (>= (Utilities|Array|Length (Variables|Default|GetAC_ActiveAbilities)) (Variables|Default|GetMaxActiveAmt)))
        (bind _returnvalue_3 (Game|AddComponentbyClass _returnvalue "/Game/Blueprints/Components/Abilities/AC_Base_ActiveAbiltiy.AC_Base_ActiveAbiltiy_C" (.name _array_element)))
        (Utilities|Array|Add (Variables|Default|GetAC_ActiveAbilities) _returnvalue_3)))))