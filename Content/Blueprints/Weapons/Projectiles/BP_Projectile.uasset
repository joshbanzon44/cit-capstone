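; BP_Projectile is a data-driven weapon projectile that deals direct-hit or splash damage.
; The construction script reads its DT_Projectiles row to set visuals, speed, splash radius, player-damage flag and multiplier-scaled damage.
; When movement stops, it messages damage to overlapping pawns or, without splash, the hit actor, then spawns impact particles and destroys itself.
; The CanDamagePlayer flag spares BP_Player only from splash, which also prints debug text.
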(event OnProjectileStop(ProjectileMovement)
  (params (ImpactResult :type Hit%20Result%20Structure%20%28by%20ref%29))
  (if (> (Variables|Default|GetSplashDamageRadius) 0.0)
    (for _array_element (Collision|GetOverlappingActors (Variables|Default|GetSplashCollision) "/Script/Engine.Pawn" :!class /Script/Engine.PrimitiveComponent)
      (if (Variables|Default|GetCanDamagePlayer)
        _
        (else
          (Utilities|Casting|CastToBP_Player _array_element
            (:CastFailed
              _))))
      (Class|BPDamagable|TakeDamage(Message) _array_element (Variables|Default|GetDamage))
      (Development|PrintString "splash"))
    (else
      (Class|BPDamagable|TakeDamage(Message) (.hitactor ImpactResult) (Variables|Default|GetDamage))))
  (Niagara|SpawnSystematLocation (Variables|Default|GetParticleSystemImpact) (Transformation|GetActorLocation))
  (Actor|DestroyActor))

(event OnSystemFinished(NiagaraSystem)
  (params (PSystem :type Niagara%20Component%20Object%20Reference)))

(event EventBeginPlay)

(event Collision|EventActorBeginOverlap
  (params (OtherActor :type Actor%20Object%20Reference)))

(event EventTick
  (params (DeltaSeconds :type Float%20%28single-precision%29)))

(event Collision|EventHit
  (params (MyComp :type Primitive%20Component%20Object%20Reference) (Other :type Actor%20Object%20Reference) (OtherComp :type Primitive%20Component%20Object%20Reference) (bSelfMoved :type Boolean) (HitLocation :type Vector :default "0, 0, 0") (HitNormal :type Vector :default "0, 0, 0") (NormalImpulse :type Vector :default "0, 0, 0") (Hit :type Hit%20Result%20Structure%20%28by%20ref%29)))

(fn ConstructionScript
  (bind _staticmesh (Variables|Default|GetStaticMesh))
  (bind _returnvalue (Utilities|GetDataTableRow "/Game/Blueprints/Weapons/Projectiles/DT_Projectiles.DT_Projectiles" (Variables|Default|GetDT_RowName))
    (:then
      (Components|StaticMesh|SetStaticMesh _staticmesh (.staticmesh _returnvalue))
      (Transformation|SetWorldScale3D _staticmesh (.meshscale _returnvalue))
      (Rendering|Material|SetMaterial _staticmesh 0 (.material _returnvalue))
      (Variables|Default|SetDamage (* (.damage _returnvalue) (Variables|Default|GetDamageMultiplier)))
      (Variables|/Script/Engine.ProjectileMovementComponent|SetInitialSpeed (Variables|Default|GetProjectileMovement) (.speed _returnvalue))
      (bind _output_get (Variables|Default|SetSplashDamageRadius (.splashradius _returnvalue)))
      (Components|Sphere|SetSphereRadius (Variables|Default|GetSplashCollision) _output_get true)
      (Variables|Default|SetCanDamagePlayer (.candamageplayer _returnvalue))
      (Class|NiagaraComponent|SetAsset (Variables|Default|GetNiagaraSystem) (.particlesystemmotion _returnvalue) true)
      (Variables|Default|SetParticleSystemImpact (.particlesystemimpact _returnvalue)))))