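; BP_Skybox is a rotating skybox actor that can switch its sky cubemap at runtime.
; The construction script applies a dynamic material with the starting sky, and Tick spins the mesh around yaw.
; ChangeSky plays a timeline forward or in reverse to animate height fog density and color plus directional and skylight intensity.
; After a short delay alongside that transition, it swaps the cubemap and rotation-speed divisor on the material.
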(event Custom|ChangeSky
  (params (SkyCubemap :type Texture%20Cube%20Object%20Reference) (SpeedDivisor :type Float%20%28double-precision%29) (Reverse :type Boolean))
  (bind _dynamicmaterial (Variables|Default|GetDynamicMaterial))
  (bind _exponentialheightfog (Variables|Default|GetExponentialHeightFog))
  (bind _component (Variables|/Script/Engine.ExponentialHeightFog|GetComponent _exponentialheightfog))
  (Utilities|FlowControl|Sequence
    (:then_0
      (if Reverse
        (bind (_direction _densityfloat _fogcolor _lightfloat) (Timeline|Fogtimeline ReverseFromEnd)
          (:Update
            (Class|ExponentialHeightFogComponent|SetFogDensity _component _densityfloat)
            (Class|ExponentialHeightFogComponent|SetFogInscatteringColor _component _fogcolor)
            (Rendering|Components|Light|SetIntensity (Variables|/Script/Engine.Light|GetLightComponent (Variables|Default|GetDirectionalLight)) _lightfloat)
            (Rendering|Components|Light|SetIntensity (Variables|/Script/Engine.SkyLight|GetLightComponent (Variables|Default|GetSkylight)) _lightfloat)))
        (else
          (Timeline|Fogtimeline PlayFromStart))))
    (:then_1
      (Utilities|FlowControl|Delay 2.5)
      (Rendering|Material|SetTextureParameterValue _dynamicmaterial "Cubemap" SkyCubemap)
      (Rendering|Material|SetScalarParameterValue _dynamicmaterial "TimeDivisorForRotationSpeed" SpeedDivisor :!class /Script/Engine.MaterialInstanceDynamic))))

(event EventBeginPlay)

(event Collision|EventActorBeginOverlap
  (params (OtherActor :type Actor%20Object%20Reference)))

(event EventTick
  (params (DeltaSeconds :type Float%20%28single-precision%29))
  (Transformation|AddWorldRotation (Variables|Default|GetStaticMeshComponent0) (Math|Rotator|MakeRotator 0.0 0.0 (* DeltaSeconds (Variables|Default|GetRotationPerSecond))) false false))

(fn ConstructionScript
  (bind _returnvalue (Rendering|Material|CreateDynamicMaterialInstance "/Game/Materials/MI_Skybox.MI_Skybox" "None" "None" :!class /Script/Engine.KismetMaterialLibrary))
  (bind _output_get (Variables|Default|SetDynamicMaterial _returnvalue))
  (Rendering|Material|SetMaterial (Variables|Default|GetStaticMeshComponent0) 0 _output_get)
  (Rendering|Material|SetTextureParameterValue (Variables|Default|GetDynamicMaterial) "Cubemap" (Variables|Default|GetStartingSky)))