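; World generator that populates a level with chests and one altar on BeginPlay.
; The current level's DT_ChestPerLevel row gives a min/max count per chest type, and chests spawn with randomized rotation at random reachable navmesh points within ChestSpawnRadius.
; The altar then spawns at a random candidate offset, discarding candidates and retrying when a chest overlap is detected.
; The construction script draws the spawn radius as a debug sphere.
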(event EventBeginPlay
  (bind _returnvalue (Transformation|GetActorLocation))
  (bind _altarspawnlocations (Variables|Default|GetAltarSpawnLocations))
  (bind (_outitem _outindex) (Utilities|Array|Random _altarspawnlocations))
  (bind _returnvalue_2 (+ _returnvalue _outitem))
  (bind _returnvalue_3 (Utilities|GetDataTableRow "/Game/DataTables/DT_ChestPerLevel.DT_ChestPerLevel" (Utilities|String|StringToName (Utilities|String|Append "Level_" (Utilities|String|ToString(Integer) (Variables|Default|GetLevel)))))
    (:then
      (bind _enumvalue (|ForEachENUM_ChestTypes)
        (:LoopBody
          (for _index (range 1 (Math|Random|RandomIntegerinRange (.minspawns (Utilities|Select :Index _enumvalue :NewEnumerator0 (.anyitem _returnvalue_3) :NewEnumerator5 (.anystatitem _returnvalue_3) :NewEnumerator1 (.rareorbetter _returnvalue_3) :NewEnumerator2 (.weapon _returnvalue_3) :NewEnumerator3 (.ability _returnvalue_3) :NewEnumerator4 (.mystic _returnvalue_3))) (.maxspawns (Utilities|Select :Index _enumvalue :NewEnumerator0 (.anyitem _returnvalue_3) :NewEnumerator5 (.anystatitem _returnvalue_3) :NewEnumerator1 (.rareorbetter _returnvalue_3) :NewEnumerator2 (.weapon _returnvalue_3) :NewEnumerator3 (.ability _returnvalue_3) :NewEnumerator4 (.mystic _returnvalue_3)))))
            (Game|SpawnActorfromClass "/Game/Blueprints/Interactables/BP_Chest.BP_Chest_C" (Math|Transform|MakeTransform (.RandomLocation (AI|Navigation|GetRandomReachablePointinRadius (Transformation|GetActorLocation) (Variables|Default|GetChestSpawnRadius) 0 0)) (CallFunction|RandomRotation) "2.000000,2.000000,2.000000") "Undefined" "MultiplyWithRoot" 0 _enumvalue 0)))
        (:then
          (bind _returnvalue_4 (Collision|SphereOverlapActors _returnvalue_2 2e+02 (Utilities|Array|MakeArray "ObjectTypeQuery11") "/Game/Blueprints/Interactables/BP_Chest.BP_Chest_C" :!label _label))
          (if _returnvalue_4
            (Utilities|Array|RemoveIndex _altarspawnlocations _outindex)
            (goto _label)
            (else
              (Game|SpawnActorfromClass "/Game/Blueprints/Interactables/BP_Altar.BP_Altar_C" (Math|Transform|MakeTransform _returnvalue_2 "0, 0, 0" "1.000000,1.000000,1.000000") "Undefined" "MultiplyWithRoot" 0 0))))))))

(fn ConstructionScript
  (Rendering|Debug|DrawDebugSphere (Transformation|GetActorLocation) (Variables|Default|GetChestSpawnRadius) 12 "(R=1.000000,G=0.104899,B=0.000000,A=1.000000)" 1.0 1e+01))

(fn RandomRotation
  (return (Math|Rotator|MakeRotator (Math|Random|RandomFloatinRange -15.0 15.0) (Math|Random|RandomFloatinRange -15.0 15.0) (Math|Random|RandomFloatinRange 0.0 3.6e+02))))