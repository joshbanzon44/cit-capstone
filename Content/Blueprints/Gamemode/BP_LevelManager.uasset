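; Level manager that spawns waves of BP_Beholder enemies around the player, starting after a delay once play begins.
; Each wave spawns a random count up to a given limit, at points 1000 units from the player in random directions.
; Bound Defeated events track live and defeated counts, triggering a delayed full-range wave when none remain or a half-range one at half the maximum or fewer.
; The SpawnEnemies function is an empty stub.
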(event Custom|OnSpawnEnemies
  (params (Range :type Integer))
  (for _index (range 1 (Math|Random|RandomIntegerinRange 1 Range))
    (bind _returnvalue (Game|SpawnActorfromClass "/Game/Blueprints/Enemies/BP_Beholder.BP_Beholder_C" (Math|Transform|MakeTransform (+ (Transformation|GetActorLocation (Variables|Default|GetPlayer)) (* (Math|Random|RandomUnitVector) 1e+03)) "0, 0, 0" "1.000000,1.000000,1.000000") "Undefined" "MultiplyWithRoot" 0 0))
    (EventDispatchers|BindEventtoDefeated _returnvalue (delegate Custom|OnEnemDeath))
    (Math|Integer|IncrementInt (Variables|Default|GetCurrentEnemyCount)
      (:%20%20
        (Development|PrintString "spawned")))))

(event Custom|OnEnemDeath
  (bind _currentenemycount (Variables|Default|GetCurrentEnemyCount))
  (Math|Integer|IncrementInt (Variables|Default|GetEnemiesDefeatedCurrentLevel)
    (:%20%20
      (Math|Integer|DecrementInt _currentenemycount
        (:%20%20
          (if (<= _currentenemycount 0)
            (Utilities|FlowControl|Delay 2.0)
            (CallFunction|OnSpawnEnemies (Variables|Default|GetMaxEnemies))
            (elif (<= (Variables|Default|GetCurrentEnemyCount) (/ (Variables|Default|GetMaxEnemies) 2))
              (Utilities|FlowControl|Delay 5.0)
              (CallFunction|OnSpawnEnemies (/ (Variables|Default|GetMaxEnemies) 2)))))))))

(event EventBeginPlay
  (bind _asbp_player (Utilities|Casting|CastToBP_Player (Game|Player|GetPlayerPawn 0)))
  (Variables|Default|SetPlayer _asbp_player)
  (Utilities|FlowControl|Delay (Variables|Default|GetLevelStartDelay))
  (CallFunction|OnSpawnEnemies (Variables|Default|GetMaxEnemies)))

(event Collision|EventActorBeginOverlap
  (params (OtherActor :type Actor%20Object%20Reference)))

(event EventTick
  (params (DeltaSeconds :type Float%20%28single-precision%29)))

(fn ConstructionScript)

(fn SpawnEnemies
  (params (Range :type Integer))
  (return 0))