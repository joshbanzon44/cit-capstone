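; BP_SaveGame is a save game data container for a wizard character's stats, loadout and appearance.
; Setter functions copy their inputs straight into its variables, with no other logic.
; SaveItemData stores the stat item inventory, weapon name, two active abilities and two passive abilities.
; SetStatMap stores the stats map, and SetColors stores the hair, inner clothing and outer clothing colors.
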(fn SaveItemData
  (params (StatItemInventory :type Map%20of%20Names%20to%20Integers) (WeaponName :type Name) (ActiveAbility1 :type Name) (ActiveAbility2 :type Name) (PassiveAbility1 :type Name) (PassiveAbility2 :type Name))
  (Variables|Default|SetStatItemInventory StatItemInventory)
  (Variables|Default|SetWeaponName WeaponName)
  (Variables|Default|SetActiveAbility1 ActiveAbility1)
  (Variables|Default|SetActiveAbility2 ActiveAbility2)
  (Variables|Default|SetPassiveAbility1 PassiveAbility1)
  (Variables|Default|SetPassiveAbility2 PassiveAbility2))

(fn SetStatMap
  (params (StatsMap :type Map%20of%20Enum_Stats%20Enums%20to%20Reals :default "NewEnumerator8"))
  (Variables|Default|SetStatsMap StatsMap))

(fn SetColors
  (params (HairColor :type Linear%20Color%20Structure) (InnerClothesColor :type Linear%20Color%20Structure) (OuterClothesColor :type Linear%20Color%20Structure))
  (Variables|Default|SetWizardColorHair HairColor)
  (Variables|Default|SetWizardColorInnerClothes InnerClothesColor)
  (Variables|Default|SetWizardColorOuterClothes OuterClothesColor))