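; Projectile launched from a chest that shows the loot's rarity and turns into an item pickup where it lands.
; On BeginPlay it rolls a rarity from weighted odds set by ChestType, launches upward with random sideways drift and picks a matching Niagara color effect.
; When the projectile stops, it spawns a stat, weapon or ability item with a random indexed row name sized from that rarity's DataTable, then destroys itself.
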(event OnProjectileStop(ProjectileMovement)
  (params (ImpactResult :type Hit%20Result%20Structure%20%28by%20ref%29))
  (bind _returnvalue (Transformation|GetActorLocation))
  (bind _rarity (Variables|Default|GetRarity))
  (bind _outrownames (DataTable|GetDataTableRowNames (Utilities|Select :Index (Variables|Default|GetRarity) :NewEnumerator0 "/Game/DataTables/DT_ItemActors_Common.DT_ItemActors_Common" :NewEnumerator1 "/Game/DataTables/DT_ItemActors_Rare.DT_ItemActors_Rare" :NewEnumerator2 "/Game/DataTables/DT_ItemActors_Epic.DT_ItemActors_Epic" :NewEnumerator3 "/Game/DataTables/DT_ItemActors_Mystic.DT_ItemActors_Mystic" :NewEnumerator4 "/Game/DataTables/DT_ItemActors_Weapon.DT_ItemActors_Weapon" :NewEnumerator5 "/Game/DataTables/DT_ItemActors_Ability_Active.DT_ItemActors_Ability_Active" :NewEnumerator6 "/Game/DataTables/DT_ItemActors_Ability_Passive.DT_ItemActors_Ability_Passive")))
  (switch Utilities|FlowControl|Switch|SwitchonEnum_Rarities (Variables|Default|GetRarity)
    (:NewEnumerator0
      (Game|SpawnActorfromClass "/Game/Blueprints/Interactables/BP_Item_Stats.BP_Item_Stats_C" (Math|Transform|MakeTransform _returnvalue "0, 0, 0" "1.000000,1.000000,1.000000") "Undefined" "MultiplyWithRoot" 0 (Utilities|String|StringToName (Utilities|String|Append "Item_" (Utilities|String|ToString(Integer) (Math|Random|RandomInteger (- (Utilities|Array|Length _outrownames) 1))))) _rarity 0 :!label _label))
    (:NewEnumerator1
      (goto _label))
    (:NewEnumerator2
      (goto _label))
    (:NewEnumerator3
      (goto _label))
    (:NewEnumerator4
      (Game|SpawnActorfromClass "/Game/Blueprints/Interactables/BP_Item_Weapon.BP_Item_Weapon_C" (Math|Transform|MakeTransform _returnvalue "0, 0, 0" "1.000000,1.000000,1.000000") "Undefined" "MultiplyWithRoot" 0 (Utilities|String|StringToName (Utilities|String|Append "Item_" (Utilities|String|ToString(Integer) (Math|Random|RandomInteger (- (Utilities|Array|Length _outrownames) 1))))) _rarity 0))
    (:NewEnumerator5
      (Game|SpawnActorfromClass "/Game/Blueprints/Interactables/BP_Item_Ability.BP_Item_Ability_C" (Math|Transform|MakeTransform _returnvalue "0, 0, 0" "1.000000,1.000000,1.000000") "Undefined" "MultiplyWithRoot" 0 false (Utilities|String|StringToName (Utilities|String|Append "Item_" (Utilities|String|ToString(Integer) (Math|Random|RandomInteger (- (Utilities|Array|Length _outrownames) 1))))) _rarity 0 :!label _label_2))
    (:NewEnumerator6
      (goto _label_2)))
  (Actor|DestroyActor))

(event EventBeginPlay
  (bind _rarity (CallFunction|GenerateRarity))
  (Variables|Default|SetRarity _rarity)
  (Variables|/Script/Engine.MovementComponent|SetVelocity (Variables|Default|GetProjectileMovement) (Math|Vector|MakeVector (Math|Random|RandomFloatinRange -1.5e+02 1.5e+02) (Math|Random|RandomFloatinRange -1.5e+02 1.5e+02) 6e+02))
  (Class|NiagaraComponent|SetAsset (Variables|Default|GetNiagara) (Utilities|Select :Index (Variables|Default|GetRarity) :NewEnumerator0 "/Game/Particles/ItemEffects/NS_ItemEffectWhite.NS_ItemEffectWhite" :NewEnumerator1 "/Game/Particles/ItemEffects/NS_ItemEffectBlue.NS_ItemEffectBlue" :NewEnumerator2 "/Game/Particles/ItemEffects/NS_ItemEffectPurple.NS_ItemEffectPurple" :NewEnumerator3 "/Game/Particles/ItemEffects/NS_ItemEffectGold.NS_ItemEffectGold" :NewEnumerator4 "/Game/Particles/ItemEffects/NS_ItemEffectRed.NS_ItemEffectRed" :NewEnumerator5 "/Game/Particles/ItemEffects/NS_ItemEffectGreen.NS_ItemEffectGreen" :NewEnumerator6 "/Game/Particles/ItemEffects/NS_ItemEffectCyan.NS_ItemEffectCyan") true))

(fn ConstructionScript)

(fn GenerateRarity
  (LocalVariables|SetRandomFloat (Math|Random|RandomFloat))
  (switch Utilities|FlowControl|Switch|SwitchonENUM_ChestTypes (Variables|Default|GetChestType)
    (:NewEnumerator0
      (if (or (<= (LocalVariables|GetRandomFloat) 0.025) (>= (LocalVariables|GetRandomFloat) 0.975))
        (return "NewEnumerator3")
        (elif (or (<= (LocalVariables|GetRandomFloat) 0.1) (>= (LocalVariables|GetRandomFloat) 0.9))
          (return "NewEnumerator2")
          (elif (or (<= (LocalVariables|GetRandomFloat) 0.25) (>= (LocalVariables|GetRandomFloat) 0.75))
            (return "NewEnumerator1")
            (elif (or (<= (LocalVariables|GetRandomFloat) 0.3) (>= (LocalVariables|GetRandomFloat) 0.7))
              (return "NewEnumerator4")
              (elif (or (<= (LocalVariables|GetRandomFloat) 0.325) (>= (LocalVariables|GetRandomFloat) 0.675))
                (return "NewEnumerator5")
                (elif (or (<= (LocalVariables|GetRandomFloat) 0.35) (>= (LocalVariables|GetRandomFloat) 0.65))
                  (return "NewEnumerator6")
                  (else
                    (return "NewEnumerator0")))))))))
    (:NewEnumerator5
      (if (or (<= (LocalVariables|GetRandomFloat) 0.025) (>= (LocalVariables|GetRandomFloat) 0.975))
        (return "NewEnumerator3")
        (elif (or (<= (LocalVariables|GetRandomFloat) 0.1) (>= (LocalVariables|GetRandomFloat) 0.9))
          (return "NewEnumerator2")
          (elif (or (<= (LocalVariables|GetRandomFloat) 0.25) (>= (LocalVariables|GetRandomFloat) 0.75))
            (return "NewEnumerator1")
            (else
              (return "NewEnumerator0"))))))
    (:NewEnumerator1
      (if (or (<= (LocalVariables|GetRandomFloat) 0.1) (>= (LocalVariables|GetRandomFloat) 0.9))
        (return "NewEnumerator3")
        (elif (or (<= (LocalVariables|GetRandomFloat) 0.25) (>= (LocalVariables|GetRandomFloat) 0.75))
          (return "NewEnumerator2")
          (else
            (return "NewEnumerator1")))))
    (:NewEnumerator2
      (return "NewEnumerator4"))
    (:NewEnumerator3
      (if (>= (LocalVariables|GetRandomFloat) 0.5)
        (return "NewEnumerator5")
        (else
          (return "NewEnumerator6"))))
    (:NewEnumerator4
      (return "NewEnumerator3"))))