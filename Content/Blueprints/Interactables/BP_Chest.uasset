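; Interactable chest that highlights on hover and opens once when activated, spawning a BP_Chest_Proj at its item spawn point.
; The construction script uses ChestType to pull mesh, materials, transform tweaks, opening animation and delay from DT_ChestActors.
; Activate clears Locked, plays the animation, waits, then passes ChestType to the spawned actor.
; GenerateRarity rolls a symmetric-threshold weighted rarity but is not called in this Blueprint.
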(event EventBeginPlay)

(event Collision|EventActorBeginOverlap
  (params (OtherActor :type Actor%20Object%20Reference)))

(event EventTick
  (params (DeltaSeconds :type Float%20%28single-precision%29)))

(event EventUnhover
  (if (not (Variables|Default|GetOpened))
    (Rendering|SetRenderCustomDepth (Variables|Default|GetSkeletalMesh) false)))

(event EventHover
  (if (not (Variables|Default|GetOpened))
    (Rendering|SetRenderCustomDepth (Variables|Default|GetSkeletalMesh) true)))

(event EventActivate
  (Variables|Default|SetLocked false)
  (if (not (or (Variables|Default|GetLocked) (Variables|Default|GetOpened)))
    (Rendering|SetRenderCustomDepth (Variables|Default|GetSkeletalMesh) false)
    (Variables|Default|SetOpened true)
    (Components|Animation|PlayAnimation (Variables|Default|GetSkeletalMesh) (Variables|Default|GetAnimToPlay) false)
    (Utilities|FlowControl|Delay (Variables|Default|GetOpeningDelay))
    (Game|SpawnActorfromClass "/Game/Blueprints/Interactables/BP_Chest_Proj.BP_Chest_Proj_C" (Math|Transform|MakeTransform (Transformation|GetWorldLocation (Variables|Default|GetItemSpawnpoint)) "0, 0, 0" "1.000000,1.000000,1.000000") "Undefined" "MultiplyWithRoot" 0 (Variables|Default|GetChestType) 0)
    (Development|PrintString "spawned")))

(fn ConstructionScript
  (bind _returnvalue (Utilities|GetDataTableRow "/Game/DataTables/DT_ChestActors.DT_ChestActors" (Utilities|Select :Index (Variables|Default|GetChestType) :NewEnumerator0 "AnyItem" :NewEnumerator5 "AnyStatItem" :NewEnumerator1 "RareOrBetter" :NewEnumerator2 "Weapon" :NewEnumerator3 "Ability" :NewEnumerator4 "Mystic"))
    (:then
      (Components|SkeletalMesh|SetSkeletalMeshAsset (Variables|Default|GetSkeletalMesh) (.mesh _returnvalue))
      (Variables|Default|SetAnimToPlay (.animation _returnvalue))
      (Transformation|SetWorldScale3D (Variables|Default|GetSkeletalMesh) (.scale _returnvalue))
      (for (_array_element _array_index) (.materials _returnvalue)
        (Rendering|Material|SetMaterial (Variables|Default|GetSkeletalMesh) _array_index _array_element))
      (Variables|Default|SetOpeningDelay (.openingdelay _returnvalue))
      (Transformation|SetRelativeLocation (Variables|Default|GetSkeletalMesh) (.meshworldoffset _returnvalue) false false))))

(fn GenerateRarity
  (LocalVariables|SetRandomFloat (Math|Random|RandomFloat))
  (if (or (<= (LocalVariables|GetRandomFloat) 0.025) (>= (LocalVariables|GetRandomFloat) 0.975))
    (return "NewEnumerator3")
    (elif (or (<= (LocalVariables|GetRandomFloat) 0.1) (>= (LocalVariables|GetRandomFloat) 0.9))
      (return "NewEnumerator2")
      (elif (or (<= (LocalVariables|GetRandomFloat) 0.25) (>= (LocalVariables|GetRandomFloat) 0.75))
        (return "NewEnumerator1")
        (else
          (return "NewEnumerator0"))))))