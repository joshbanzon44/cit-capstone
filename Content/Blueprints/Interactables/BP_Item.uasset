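; BP_Item is an interactable world pickup with a rarity tier that bobs up and down on a timeline and spins continuously.
; The construction script reads a named row from the rarity's data table to set mesh, scale, rotation and materials, and picks a rarity-colored Niagara effect.
; Hover and Unhover toggle custom depth on the mesh for highlighting.
; Activate only prints a placeholder message instead of collecting the item.
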(event EventBeginPlay
  (bind _bounceheight (Variables|Default|GetBounceHeight))
  (Variables|Default|SetStartLocation (Variables|/Script/Engine.SceneComponent|GetRelativeLocation (Variables|Default|GetStaticMesh)))
  (bind _0_1_0 (Timeline|Timeline010 Play)
    (:Update
      (Transformation|SetRelativeLocation (Variables|Default|GetStaticMesh) (Math|Vector|Lerp(Vector) (- (Variables|Default|GetStartLocation) (Math|Vector|MakeVector 0.0 0.0 _bounceheight)) (+ (Variables|Default|GetStartLocation) (Math|Vector|MakeVector 0.0 0.0 _bounceheight)) _0_1_0) false false))))

(event Collision|EventActorBeginOverlap
  (params (OtherActor :type Actor%20Object%20Reference)))

(event EventTick
  (params (DeltaSeconds :type Float%20%28single-precision%29))
  (Class|Actor|AddActorWorldRotation (Math|Rotator|MakeRotator 0.0 0.0 (* DeltaSeconds (Variables|Default|GetRotationDegreesPerSecond)))))

(event EventHover
  (Rendering|SetRenderCustomDepth (Variables|Default|GetStaticMesh) true))

(event EventUnhover
  (Rendering|SetRenderCustomDepth (Variables|Default|GetStaticMesh) false))

(event EventActivate
  (Development|PrintString "collect item and add to player"))

(fn ConstructionScript
  (bind _staticmesh (Variables|Default|GetStaticMesh))
  (bind _returnvalue (Utilities|GetDataTableRow (Utilities|Select :Index (Variables|Default|GetRarity) :NewEnumerator0 "/Game/DataTables/DT_ItemActors_Common.DT_ItemActors_Common" :NewEnumerator1 "/Game/DataTables/DT_ItemActors_Rare.DT_ItemActors_Rare" :NewEnumerator2 "/Game/DataTables/DT_ItemActors_Epic.DT_ItemActors_Epic" :NewEnumerator3 "/Game/DataTables/DT_ItemActors_Mystic.DT_ItemActors_Mystic") (Variables|Default|GetDT_RowName))
    (:then
      (bind _output_get (Variables|Default|SetSTR_ItemActor _returnvalue))
      (Components|StaticMesh|SetStaticMesh _staticmesh (.mesh _output_get))
      (Transformation|SetWorldScale3D _staticmesh (.meshscale _output_get))
      (Transformation|SetWorldRotation _staticmesh (.meshrotation _output_get) false false)
      (for (_array_element _array_index) (.materials _output_get)
        (Rendering|Material|SetMaterial _staticmesh _array_index _array_element))
      (Class|NiagaraComponent|SetAsset (Variables|Default|GetNiagara) (Utilities|Select :Index (Variables|Default|GetRarity) :NewEnumerator0 "/Game/Particles/NS_ItemEffectWhite.NS_ItemEffectWhite" :NewEnumerator1 "/Game/Particles/NS_ItemEffectBlue.NS_ItemEffectBlue" :NewEnumerator2 "/Game/Particles/NS_ItemEffectPurple.NS_ItemEffectPurple" :NewEnumerator3 "/Game/Particles/NS_ItemEffectGold.NS_ItemEffectGold") true))))