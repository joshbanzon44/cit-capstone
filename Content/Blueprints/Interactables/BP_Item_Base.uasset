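; Base pickup actor for collectible items, weapons and abilities that bobs on a timeline, spins each tick and toggles custom depth on hover.
; The construction script uses Rarity to pick the data table for mesh, transform and materials, a color-coded Niagara effect, and the stats table that supplies the display name.
; On Activate it passes itself to the player's CollectItem, calls CallItemCollected and destroys itself.
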(event EventBeginPlay
  (bind _bounceheight (Variables|Default|GetBounceHeight))
  (Variables|Default|SetStartLocation (Variables|/Script/Engine.SceneComponent|GetRelativeLocation (Variables|Default|GetStaticMesh)))
  (bind _0_1_0 (Timeline|Timeline Play)
    (:Update
      (Transformation|SetRelativeLocation (Variables|Default|GetStaticMesh) (Math|Vector|Lerp(Vector) (- (Variables|Default|GetStartLocation) (Math|Vector|MakeVector 0.0 0.0 _bounceheight)) (+ (Variables|Default|GetStartLocation) (Math|Vector|MakeVector 0.0 0.0 _bounceheight)) _0_1_0) false false))))

(event EventTick
  (params (DeltaSeconds :type Float%20%28single-precision%29))
  (Class|Actor|AddActorWorldRotation (Math|Rotator|MakeRotator 0.0 0.0 (* DeltaSeconds (Variables|Default|GetRotationDegreesPerSecond)))))

(event EventHover
  (Rendering|SetRenderCustomDepth (Variables|Default|GetStaticMesh) true))

(event EventUnhover
  (Rendering|SetRenderCustomDepth (Variables|Default|GetStaticMesh) false))

(event EventActivate
  (params (IsMainInteract :type Boolean))
  (bind _asbp_player (Utilities|Casting|CastToBP_Player (Game|Player|GetPlayerPawn 0)))
  (Default|CollectItem _asbp_player (.name (Variables|Default|GetSTR_ItemActor)) self (Transformation|GetActorLocation) IsMainInteract)
  (Default|CallItemCollected)
  (Actor|DestroyActor))

(fn ConstructionScript
  (bind _rarity (Variables|Default|GetRarity))
  (bind _staticmesh (Variables|Default|GetStaticMesh))
  (bind _returnvalue (Utilities|Select :Index _rarity :NewEnumerator0 "/Game/DataTables/DT_ItemStats.DT_ItemStats" :NewEnumerator1 "/Game/DataTables/DT_ItemStats.DT_ItemStats" :NewEnumerator2 "/Game/DataTables/DT_ItemStats.DT_ItemStats" :NewEnumerator3 "/Game/DataTables/DT_ItemStats.DT_ItemStats" :NewEnumerator4 "/Game/DataTables/DT_Weapons.DT_Weapons" :NewEnumerator5 "/Game/DataTables/DT_Ability_Active.DT_Ability_Active" :NewEnumerator6 "/Game/DataTables/DT_Ability_Passive.DT_Ability_Passive"))
  (bind _returnvalue_2 (Utilities|GetDataTableRow (Utilities|Select :Index (Variables|Default|GetRarity) :NewEnumerator0 "/Game/DataTables/DT_ItemActors_Common.DT_ItemActors_Common" :NewEnumerator1 "/Game/DataTables/DT_ItemActors_Rare.DT_ItemActors_Rare" :NewEnumerator2 "/Game/DataTables/DT_ItemActors_Epic.DT_ItemActors_Epic" :NewEnumerator3 "/Game/DataTables/DT_ItemActors_Mystic.DT_ItemActors_Mystic" :NewEnumerator4 "/Game/DataTables/DT_ItemActors_Weapon.DT_ItemActors_Weapon" :NewEnumerator5 "/Game/DataTables/DT_ItemActors_Ability_Active.DT_ItemActors_Ability_Active" :NewEnumerator6 "/Game/DataTables/DT_ItemActors_Ability_Passive.DT_ItemActors_Ability_Passive") (Variables|Default|GetDT_RowName))
    (:then
      (bind _output_get (Variables|Default|SetSTR_ItemActor _returnvalue_2))
      (Variables|Default|SetItemName (.name _output_get))
      (Components|StaticMesh|SetStaticMesh _staticmesh (.mesh _output_get))
      (Transformation|SetRelativeLocation _staticmesh (+ (.meshpositionoffset _output_get) (Variables|/Script/Engine.SceneComponent|GetRelativeLocation _staticmesh)) false false)
      (Transformation|SetWorldScale3D _staticmesh (.meshscale _output_get))
      (Transformation|SetWorldRotation _staticmesh (.meshrotation _output_get) false false)
      (for (_array_element _array_index) (.materials _output_get)
        (Rendering|Material|SetMaterial _staticmesh _array_index _array_element))
      (Class|NiagaraComponent|SetAsset (Variables|Default|GetNiagara) (Utilities|Select :Index (Variables|Default|GetRarity) :NewEnumerator0 "/Game/Particles/ItemEffects/NS_ItemEffectWhite.NS_ItemEffectWhite" :NewEnumerator1 "/Game/Particles/ItemEffects/NS_ItemEffectBlue.NS_ItemEffectBlue" :NewEnumerator2 "/Game/Particles/ItemEffects/NS_ItemEffectPurple.NS_ItemEffectPurple" :NewEnumerator3 "/Game/Particles/ItemEffects/NS_ItemEffectGold.NS_ItemEffectGold" :NewEnumerator4 "/Game/Particles/ItemEffects/NS_ItemEffectRed.NS_ItemEffectRed" :NewEnumerator5 "/Game/Particles/ItemEffects/NS_ItemEffectGreen.NS_ItemEffectGreen" :NewEnumerator6 "/Game/Particles/ItemEffects/NS_ItemEffectGreen.NS_ItemEffectGreen") true)
      (if (or (Utilities|Enum|Equal(Enum) (Variables|Default|GetRarity) "NewEnumerator5") (Utilities|Enum|Equal(Enum) (Variables|Default|GetRarity) "NewEnumerator6"))
        (bind _returnvalue_3 (Utilities|GetDataTableRow _returnvalue (Variables|Default|GetItemName))
          (:then
            (Variables|Default|SetVisibleName (.Name (Utilities|Struct|BreakSTR_AbilityStats _returnvalue_3)))))
        (elif (Utilities|Enum|Equal(Enum) (Variables|Default|GetRarity) "NewEnumerator4")
          (bind _returnvalue_4 (Utilities|GetDataTableRow _returnvalue (Variables|Default|GetItemName))
            (:then
              (Variables|Default|SetVisibleName (.Name (Utilities|Struct|BreakSTR_WeaponClass _returnvalue_4)))))
          (else
            (bind _returnvalue_5 (Utilities|GetDataTableRow _returnvalue (Variables|Default|GetItemName))
              (:then
                (Variables|Default|SetVisibleName (.Name (Utilities|Struct|BreakSTR_ItemStats _returnvalue_5)))))))))))