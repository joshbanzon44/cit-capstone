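; BP_Altar is a boss altar that starts a boss fight when its child boss item is collected and opens the stage exit portal afterwards.
; On BeginPlay it caches the skybox, current stage and player controller, then traces down to sit slightly sunk into the ground, aligned to the surface normal.
; Collection swaps sky and music and spawns BP_Boss; its defeat reverses the sky, changes music and opens BP_Portal.
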(event Custom|OnBossItemCollected
  (bind _roguecontroller (Variables|Default|GetRogueController))
  (bind _backgroundmusic (Variables|/Game/Blueprints/Gamemode/RoguePlayerController.RoguePlayerController_C|GetBackgroundMusic _roguecontroller))
  (Default|ChangeSky (Variables|Default|GetSkybox) "/Game/Textures/TC_Space.TC_Space" 2e+04 false (Variables|Default|GetCurrent%20Stage) 0.1)
  (Audio|Components|Audio|FadeOut _backgroundmusic 2.0 0.0 "Linear" :!class /Script/Engine.AudioComponent)
  (Utilities|FlowControl|Delay 2.0)
  (Audio|Components|Audio|SetSound _backgroundmusic "/Game/Audio/Sounds/Music/SFX_LandOfMystery.SFX_LandOfMystery")
  (Audio|Components|Audio|FadeIn _backgroundmusic 2.0 1.0 0.0 "Linear" :!class /Script/Engine.AudioComponent)
  (Utilities|FlowControl|Delay 2.0)
  (bind _returnvalue (Game|SpawnActorfromClass "/Game/Blueprints/Enemies/BP_Boss.BP_Boss_C" (Math|Transform|MakeTransform (Transformation|GetWorldLocation (Variables|Default|GetBossSpawnpoint)) "0, 0, 0" "1.000000,1.000000,1.000000") "Undefined" "MultiplyWithRoot" 0 0 0))
  (EventDispatchers|BindEventtoDefeatedBoss _returnvalue (delegate Custom|OnBossDefeated)))

(event Custom|OnBossDefeated
  (bind _roguecontroller (Variables|Default|GetRogueController))
  (bind _backgroundmusic (Variables|/Game/Blueprints/Gamemode/RoguePlayerController.RoguePlayerController_C|GetBackgroundMusic _roguecontroller))
  (Default|ChangeSky (Variables|Default|GetSkybox) (Variables|Default|GetSky%20Cubemap) 2e+04 true (Variables|Default|GetCurrent%20Stage) 0.5)
  (Audio|Components|Audio|FadeOut _backgroundmusic 2.0 0.0 "Linear" :!class /Script/Engine.AudioComponent)
  (bind _outactors (Actor|GetAllActorsOfClass "/Game/Blueprints/Interactables/BP_Portal.BP_Portal_C"))
  (Default|OpenPortal (Utilities|Array|Get(acopy) _outactors))
  (Audio|Components|Audio|SetSound _backgroundmusic "/Game/Audio/Sounds/Music/SFX_EnchantedForest.SFX_EnchantedForest")
  (Audio|Components|Audio|FadeIn _backgroundmusic 2.0 1.0 0.0 "Linear" :!class /Script/Engine.AudioComponent))

(event EventBeginPlay
  (bind _returnvalue (Transformation|GetActorLocation))
  (bind _returnvalue_2 (- _returnvalue "0.000000,0.000000,-1.000000"))
  (bind _outactors (Actor|GetAllActorsOfClass "/Game/Blueprints/Gamemode/BP_Skybox.BP_Skybox_C"))
  (Variables|Default|SetSkybox (Utilities|Array|Get(acopy) _outactors))
  (bind _asbp_item_base (Utilities|Casting|CastToBP_Item_Base (Variables|/Script/Engine.ChildActorComponent|GetChildActor (Variables|Default|GetBossItem))))
  (EventDispatchers|BindEventtoItemCollected _asbp_item_base (delegate Custom|OnBossItemCollected))
  (Utilities|FlowControl|DelayUntilNextTick)
  (bind _asrogue_gamemode (Utilities|Casting|CastToRogueGamemode (Game|GetGameMode))
    (:then
      (Variables|Default|SetCurrent%20Stage (Variables|/Game/Blueprints/Gamemode/BP_SaveGame.BP_SaveGame_C|GetCurrentStage (Variables|/Game/Blueprints/Gamemode/RogueGamemode.RogueGamemode_C|GetSaveGame _asrogue_gamemode))))
    (:CastFailed
      _))
  (bind _outhit (Collision|LineTraceByChannel _returnvalue_2 (+ _returnvalue_2 "0.000000,0.000000,-200.000000") "TraceTypeQuery1" false 0 "None"))
  (Transformation|SetActorLocationAndRotation (- (.Location (Collision|BreakHitResult _outhit)) (Math|Vector|MakeVector 0.0 0.0 (Math|Random|RandomFloatinRange 5.0 15.0))) (Math|Rotator|MakeRotfromZ (.ImpactNormal (Collision|BreakHitResult _outhit))))
  (bind _asrogue_player_controller (Utilities|Casting|CastToRoguePlayerController (Game|GetPlayerController 0)))
  (Variables|Default|SetRogueController _asrogue_player_controller))

(fn ConstructionScript)